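; BP_TetrisGameMode is the Tetris game mode that switches UI screens and relays game flow events.
; BPFStartGame clears all widgets, shows the operation guide widget, tells BP_TetrisController to start the game, then refreshes the score.
; BPFUpdateScore forwards score refreshes to that stored guide widget, and BPFGameOver replaces all widgets with the game over screen.
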(event `self.BPF_StartGame`
  (`WidgetLayoutLibrary.RemoveAllWidgets`)
  (bind _returnvalue (`|CreateWidget` "/Game/HUD/Widget_OperationGuide.Widget_OperationGuide_C"))
  (bind _output_get (set `self.OperationWidget` _returnvalue))
  (`UserWidget.AddToViewport` _output_get 0)
  (bind _asbp_tetris_controller (cast `/Game/GameBase/BP_TetrisController` (`GameplayStatics.GetPlayerController` 0)))
  (`TetrisController.StartGame` _asbp_tetris_controller)
  (`/Game/HUD/Widget_OperationGuide.UpdateScore` (`self.OperationWidget`)))

(event `self.BPF_UpdateScore`
  (`/Game/HUD/Widget_OperationGuide.UpdateScore` (`self.OperationWidget`)))

(event `self.BPF_GameOver`
  (`WidgetLayoutLibrary.RemoveAllWidgets`)
  (bind _returnvalue (`|CreateWidget` "/Game/HUD/Widget_GameOver.Widget_GameOver_C"))
  (`UserWidget.AddToViewport` _returnvalue 0))

(fn `UserConstructionScript`)